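; Advanced water Blueprint that computes a Gerstner-style vertical wave offset at a given world position.
; GetGerstnerWaveOffsetZ sums four GerstnerWave results, with per-wave parameters packed into vector components and two directions per Direction vector.
; Each wave is a sine of position projected onto its normalized direction plus a game-time phase, scaled by steepness, amplitude, wavelength and wave count.
; Event graph and construction script are empty.
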(fn `Gerstner Wave`
  (params (Stepness :type "Float (double-precision)") (NumberOfWaves :type "Float (double-precision)") (Amplitude :type "Float (double-precision)") (Direction :type "Vector2D Structure") (WorldPosition :type "Vector Structure") (WaveLenght :type "Float (double-precision)") (Speed :type "Float (double-precision)"))
  (returns (zHeight :type "Float (double-precision)"))
  (bind _returnvalue (/ 6.283 WaveLenght))
  (return (* (/ Stepness (* _returnvalue NumberOfWaves Amplitude)) (* (`KismetMathLibrary.Sin` (+ (* (`KismetMathLibrary.DotProduct2D` (`KismetMathLibrary.Normal2D` Direction) (`KismetMathLibrary.MakeVector2D` (.x WorldPosition) (.y WorldPosition))) _returnvalue) (* (* _returnvalue Speed) (`KismetSystemLibrary.GetGameTimeInSeconds`)))) (* _returnvalue Amplitude)))))

(fn `GetGerstnerWaveOffsetZ`
  (params (WorldPosition :type "Vector Structure"))
  (returns (zHeight :type "Float (double-precision)"))
  (bind (_x _y _z _w) (`KismetMathLibrary.BreakVector4` (`self.Direction1`)))
  (bind (_x_2 _y_2 _z_2 _w_2) (`KismetMathLibrary.BreakVector4` (`self.Direction`)))
  (bind (_x_3 _y_3 _z_3 _w_3) (`KismetMathLibrary.BreakVector4` (`self.Speeds`)))
  (bind (_x_4 _y_4 _z_4 _w_4) (`KismetMathLibrary.BreakVector4` (`self.WaveLenght`)))
  (bind (_x_5 _y_5 _z_5 _w_5) (`KismetMathLibrary.BreakVector4` (`self.Stepnesses`)))
  (bind (_x_6 _y_6 _z_6 _w_6) (`KismetMathLibrary.BreakVector4` (`self.Amplitudes`)))
  (bind _zheight (`self.Gerstner Wave` _x_5 0.0 _x_6 (`KismetMathLibrary.MakeVector2D` _x_2 _y_2) WorldPosition _x_4 _x_3))
  (bind _zheight_2 (`self.Gerstner Wave` _y_5 0.0 _y_6 (`KismetMathLibrary.MakeVector2D` _z_2 _w_2) WorldPosition _y_4 _y_3))
  (bind _zheight_3 (`self.Gerstner Wave` _z_5 0.0 _z_6 (`KismetMathLibrary.MakeVector2D` _x _y) WorldPosition _z_4 _z_3))
  (bind _zheight_4 (`self.Gerstner Wave` _w_5 0.0 _w_6 (`KismetMathLibrary.MakeVector2D` _z _w) WorldPosition _w_4 _w_3))
  (return (+ _zheight _zheight_2 _zheight_3 _zheight_4)))

(fn `UserConstructionScript`)